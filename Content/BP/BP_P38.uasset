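; BP_P38 is a player-flown aircraft pawn, apparently a P-38, with roll, pitch, boost and twin-missile fire.
; Tick feeds movement input along the forward vector scaled by Boost, while axis inputs apply frame-rate-scaled local rotations.
; BeginPlay registers Left and Right with a rotating mesh component, and Fire triggers BPLauncher from two Body sockets.
; Boost press sets Boost, but release sets a separate Speed variable, leaving Boost unchanged.
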(event EventBeginPlay
  (Default|AddSceneComponent (Variables|Default|GetBP_RotatingStaticMeshComponent) (Variables|Default|GetLeft))
  (Default|AddSceneComponent (Variables|Default|GetBP_RotatingStaticMeshComponent) (Variables|Default|GetRight)))

(event EventTick
  (params (DeltaSeconds :type Float%20%28single-precision%29))
  (Pawn|Input|AddMovementInput (Transformation|GetActorForwardVector) (Variables|Default|GetBoost) false))

(event Input|ActionEvents|InputActionBoost
  (params (Key :type Key%20Structure :default "None"))
  (:Pressed
    (Variables|Default|SetBoost 1.0))
  (:Released
    (Variables|Default|SetSpeed 0.5)))

(event Input|ActionEvents|InputActionFire
  (params (Key :type Key%20Structure :default "None"))
  (:Pressed
    (Default|Launch (Variables|Default|GetBP_Launcher) (Utilities|Struct|MakeRigVMFunction_MathTransformTransformVector "0.000000,0.000000,0.000000|0.000000,0.000000,-0.000000|1.000000,1.000000,1.000000" (Transformation|GetSocketLocation (Variables|Default|GetBody) "missle1")))
    (Default|Launch (Variables|Default|GetBP_Launcher) (Utilities|Struct|MakeRigVMFunction_MathTransformTransformVector "0.000000,0.000000,0.000000|0.000000,0.000000,-0.000000|1.000000,1.000000,1.000000" (Transformation|GetSocketLocation (Variables|Default|GetBody) "missle2")))))

(event Input|AxisEvents|InputAxisPitch
  (params (AxisValue :type Float%20%28single-precision%29))
  ;[1 1 1] Pitch
  (Transformation|AddActorLocalRotation (Math|Rotator|MakeRotator 0.0 (* AxisValue (Variables|Default|GetRotationSpeed) (Utilities|Time|GetWorldDeltaSeconds)) 0.0) false false))

(event Input|AxisEvents|InputAxisRoll
  (params (AxisValue :type Float%20%28single-precision%29))
  ;[1 1 1] Roll
  (Transformation|AddActorLocalRotation (Math|Rotator|MakeRotator (* AxisValue (Variables|Default|GetRotationSpeed) (Utilities|Time|GetWorldDeltaSeconds)) 0.0 0.0) false false))

(fn ConstructionScript)